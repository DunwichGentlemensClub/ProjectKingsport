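; Priest unit Blueprint whose ability lures enemy Workers toward it.
; Activating the ability finds Workers overlapping the AbilityRadius component and, on the server only, orders those on other teams to move to the Priest's current location.
; It also overrides the team material setup, applying a blue or red material to its static mesh based on TeamIndex.
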(event `self.SetMaterialFromTeam`
  ;[1 0 0.6564] Init Material (Override)
  (bind _asmaterial (cast `Material` (`KismetMathLibrary.SelectObject` "/Game/Materials/Blue.Blue" "/Game/Materials/Red.Red" (== (`self.TeamIndex`) 0))))
  (`PrimitiveComponent.SetMaterial` (`self.StaticMesh`) 0 _asmaterial))

(event `self.ActivateAbility`
  (`self.DistractNearbyEnemyWorkers`))

(fn `DistractNearbyEnemyWorkers`
  (for _array_element (`PrimitiveComponent.GetOverlappingActors` (`self.AbilityRadius`) "/Game/Blueprints/Characters/Worker.Worker_C")
    (bind _asworker (cast `/Game/Blueprints/Characters/Worker` _array_element))
    (if (!= (`/Game/Blueprints/Characters/Unit.TeamIndex` _asworker) (`self.TeamIndex`))
      (`/Engine/EditorBlueprintResources/ActorMacros.Switch Has Authority`
        (:`Authority`
          (`self.MoveUnit` _asworker (`self.K2_GetActorLocation`) null))))))

(fn `UserConstructionScript`
  (`parent.UserConstructionScript`))