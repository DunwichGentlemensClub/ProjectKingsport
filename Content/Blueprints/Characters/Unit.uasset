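; Unit is a selectable character that marks selection with a point light and moves on command.
; OnSelected and OnDeselected switch the light's intensity on and off, and the construction script starts it dark.
; MoveUnit sends the unit to a goal location through its AI controller's MoveToLocation with a small acceptance radius.
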(event `OnSelected`
  (`LightComponent.SetIntensity` (`self.PointLight`) 10000.0))

(event `OnDeselected`
  (`LightComponent.SetIntensity` (`self.PointLight`) 0.0))

(event `MoveUnit`
  (params (Goal :type "Vector Structure"))
  (`AIController.MoveToLocation` (`AIBlueprintHelperLibrary.GetAIController` self) Goal 10.0 true true false true null true))

(fn `UserConstructionScript`
  (`LightComponent.SetIntensity` (`self.PointLight`) 0.0))