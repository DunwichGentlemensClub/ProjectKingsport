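; Worker character Blueprint that moves the unit to a goal location or to a free access point on a targeted Building.
; MoveUnit releases any held access point, then requests a free one when the hit actor casts to Building and redirects the move to its world location.
; Its AI controller performs the move, which is skipped if a targeted Building has no free access point.
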(event `self.MoveUnit`
  (params (Goal :type "Vector Structure") (HitActor :type "Actor Object Reference"))
  (if (`self.HasAccessPoint`)
    (set `/Game/Blueprints/Components/AccessPoint.IsOccupied` false (`self.CurrentAccessPoint`))
    (set `self.HasAccessPoint` false))
  (set `self.MoveLocation` Goal)
  (bind _asbuilding (cast `/Game/Blueprints/Building` HitActor)
    (:`then`
      (bind (_accesspointref _foundaccesspoint) (`/Game/Blueprints/Building.GetFreeAccessPoint` _asbuilding))
      (if _foundaccesspoint
        (bind _output_get (set `self.CurrentAccessPoint` _accesspointref))
        (set `self.HasAccessPoint` true)
        (set `self.MoveLocation` (`SceneComponent.K2_GetComponentLocation` _output_get))
        (`AIController.MoveToLocation` (`AIBlueprintHelperLibrary.GetAIController` self) (`self.MoveLocation`) -1.0 true true false true null true :!label _label)))
    (:`CastFailed`
      (goto _label))))

(fn `UserConstructionScript`
  (`parent.UserConstructionScript`))