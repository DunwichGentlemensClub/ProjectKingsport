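; RTS player controller that drives a CameraPawn and handles click-based unit selection and movement orders.
; Each tick, input axes pan the pawn through its floating movement and zoom the spring arm within bounds, with pitch remapped from arm length so the view tilts as it zooms.
; PrimaryClick traces under the cursor to select a Unit, otherwise it sends the current unit to the Visibility-trace hit location.
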(event `self.ReceiveBeginPlay`
  (bind _ascamera_pawn (cast `/Game/Blueprints/CameraPawn` (`self.K2_GetPawn`)))
  (set `self.CameraPawn` _ascamera_pawn))

(event `self.ReceiveTick`
  (params (DeltaSeconds :type "Float (single-precision)"))
  (bind (_zoomboundaries_x _zoomboundaries_y) (`KismetMathLibrary.BreakVector2D` (`self.ZoomBoundaries`)))
  (bind (_zoomboundaries_x_2 _zoomboundaries_y_2) (`KismetMathLibrary.BreakVector2D` (`self.ZoomBoundaries`)))
  (bind _cameraspeed (`self.CameraSpeed`))
  (bind _rootcomponent (`Actor.RootComponent` (`self.CameraPawn`)))
  (bind _springarm (`/Game/Blueprints/CameraPawn.SpringArm` (`self.CameraPawn`)))
  (bind (_returnvalue_roll _returnvalue_pitch _returnvalue_yaw) (`KismetMathLibrary.BreakRotator` (`SceneComponent.K2_GetComponentRotation` _rootcomponent)))
  ;[1 1 1] Camera Control
  (`PawnMovementComponent.AddInputVector` (`/Game/Blueprints/CameraPawn.FloatingPawnMovement` (`self.CameraPawn`)) (`KismetMathLibrary.MakeVector` (* _cameraspeed (`self.GetInputAxisValue`)) (* _cameraspeed (`self.GetInputAxisValue`))) false)
  (bind _output_get (set `SpringArmComponent.TargetArmLength` (`KismetMathLibrary.FClamp` (+ (* (`KismetMathLibrary.FClamp` (`self.GetInputAxisValue`) -1.0) (`self.ZoomSpeed`)) (`SpringArmComponent.TargetArmLength` _springarm)) _zoomboundaries_x _zoomboundaries_y) _springarm))
  (`SceneComponent.K2_SetWorldRotation` _rootcomponent (`KismetMathLibrary.MakeRotator` _returnvalue_roll (`KismetMathLibrary.MapRangeClamped` _output_get _zoomboundaries_x_2 _zoomboundaries_y_2 75.0 15.0) _returnvalue_yaw) false false))

(event `InputAction|PrimaryClick`
  (params (Key :type "Key Structure"))
  (bind _currentunit (`self.CurrentUnit`))
  (:`Pressed`
    (bind _asunit (cast `/Game/Blueprints/Characters/Unit` (`.HitActor` (`GameplayStatics.BreakHitResult` (`self.GetHitResultUnderCursorByChannel` "TraceTypeQuery3"))))
      (:`then`
        (set `self.CurrentUnit` _asunit))
      (:`CastFailed`
        (if (`KismetSystemLibrary.IsValid` _currentunit)
          (`/Game/Blueprints/Characters/Unit.MoveUnit` _currentunit (`.Location` (`GameplayStatics.BreakHitResult` (`self.GetHitResultUnderCursorByChannel` "TraceTypeQuery1")))))))))

(fn `UserConstructionScript`)