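; RTS HUD that draws a drag-selection box and collects the Units inside it.
; StartRect anchors the box at the mouse position cached each Tick, and StopRect ends the drag.
; While dragging, DrawHUD draws the outline with four lines via Draw2DBox, refreshes SelectedUnits through GetActorsInSelectionRectangle, and prints the mouse position.
; BeginPlay caches the RTSController.
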(event `self.ReceiveBeginPlay`
  (bind _asrtscontroller (cast `/Game/Blueprints/RTSController` (`GameplayStatics.GetPlayerController` 0)))
  (set `self.Controller` _asrtscontroller))

(event `self.ReceiveDrawHUD`
  (params (SizeX :type Integer) (SizeY :type Integer))
  (bind _mousepos (`self.MousePos`))
  (if (`self.IsDrawingRect`)
    (`self.Draw2DBox` (stale `StartRect` _output_get) _mousepos 3.0 (struct :`R` 0.485349 :`G` 0.501 :`A` 1.0))
    (set `self.SelectedUnits` (`self.GetActorsInSelectionRectangle` "/Game/Blueprints/Characters/Unit.Unit_C" (`self.RectStartPoint`) _mousepos false))
    (`KismetSystemLibrary.PrintString` (`KismetStringLibrary.Conv_Vector2dToString` _mousepos))))

(event `StartRect`
  (set `self.IsDrawingRect` true)
  (bind _output_get (set `self.RectStartPoint` (`self.MousePos`))))

(event `StopRect`
  (set `self.IsDrawingRect` false))

(event `self.ReceiveTick`
  (params (DeltaSeconds :type "Float (single-precision)"))
  (bind (_locationx _locationy) (`PlayerController.GetMousePosition` (`GameplayStatics.GetPlayerController` 0)))
  (set `self.MousePos` (`KismetMathLibrary.MakeVector2D` _locationx _locationy)))

(fn `Draw2DBox`
  (params (StartPoint :type "Vector2D Structure") (EndPoint :type "Vector2D Structure") (Thickness :type "Float (double-precision)") (Color :type "LinearColor Structure"))
  (bind (_x _y) (`KismetMathLibrary.BreakVector2D` StartPoint))
  (bind (_x_2 _y_2) (`KismetMathLibrary.BreakVector2D` EndPoint))
  (`self.DrawLine` _x _y _x_2 _y Color Thickness)
  (`self.DrawLine` _x _y _x _y_2 Color Thickness)
  (`self.DrawLine` _x _y_2 _x_2 _y_2 Color Thickness)
  (`self.DrawLine` _x_2 _y _x_2 _y_2 Color Thickness)
  (return))

(fn `UserConstructionScript`)